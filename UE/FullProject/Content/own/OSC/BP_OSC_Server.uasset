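; OSC server actor that receives hand-tracking bundles and turns them into gesture and motion state for two hands.
; On BeginPlay it starts listening on a local or LED-screen IP, then after a short delay broadcasts setup completion and binds the bundle handler.
; Each message's position in the bundle selects the hand and field to write in the Hands array, with X negated.
; Debug prints report message count and optionally Hands[1] state.
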(event Custom|OSC_Bundle_Received
  (params (Bundle :type OSC%20Bundle%20Structure%20%28by%20ref%29) (IPAddress :type String) (Port :type Integer))
  (CallFunction|HandleIncomingBundle Bundle)
  (Math|Integer|IncrementInt (Variables|Default|GetMessageIndex)
    (:%20%20
      (CallFunction|Printinfo))))

(event EventBeginPlay
  (bind _osc_gestureserver (Variables|Server|GetOSC_GestureServer))
  (CallFunction|SetupOSCServer)
  (Utilities|FlowControl|Delay 0.2)
  (Default|CallOnOSCSetupComplete _osc_gestureserver)
  (EventDispatchers|BindEventtoOnOscBundleReceived _osc_gestureserver (EventDispatchers|CreateEvent :!event Custom|OSC_Bundle_Received)))

(event Collision|EventActorBeginOverlap
  (params (OtherActor :type Actor%20Object%20Reference)))

(event EventTick
  (params (DeltaSeconds :type Float%20%28single-precision%29)))

(fn ConstructionScript)

(fn SetupOSCServer
  (if (Variables|Server|GetIsLocal_IP?)
    (bind _returnvalue (Class|OSCManager|CreateOSCServer (Variables|Server|GetLocalNetwork_IP) 3002 false true "GestureServer" 0))
    (bind _output_get (Variables|Server|SetOSC_GestureServer _returnvalue))
    (Development|PrintString (Utilities|String|Append "Created Server \"" (Utilities|GetDisplayName _output_get) "\" on IP: " (Variables|Server|GetLocalNetwork_IP)) true true "(R=0.000000,G=1.000000,B=0.044866,A=1.000000)" 1e+01)
    (return)
    (else
      (bind _returnvalue_2 (Class|OSCManager|CreateOSCServer (Variables|Server|GetLED_Screen_DAE_IP) 3002 false true "GestureServer" 0))
      (bind _output_get_2 (Variables|Server|SetOSC_GestureServer _returnvalue_2))
      (Development|PrintString (Utilities|String|Append "Created Server \"" (Utilities|GetDisplayName _output_get_2) "\" on IP: " (Variables|Server|GetLED_Screen_DAE_IP)) true true "(R=0.000000,G=1.000000,B=0.044866,A=1.000000)" 1e+01)
      (return))))

(fn CheckHandParameters
  (params (Index :type Integer) (Value :type Float%20%28double-precision%29) (StartingIndex :type Integer) (AmountOfIndexes :type Integer) (HandNR :type Integer))
  (bind _returnvalue (- Index StartingIndex))
  (bind _hands (Variables|Default|GetHands))
  (bind _output (Utilities|Array|Get(acopy) _hands HandNR))
  (if (and (>= _returnvalue 0) (< _returnvalue AmountOfIndexes))
    (switch int _returnvalue
      (:0
        (Utilities|Struct|SetmembersinS_HandValues (.values _output) Value))
      (:1
        (Utilities|Struct|SetmembersinS_HandValues (.values _output) Value))
      (:2
        (Utilities|Struct|SetmembersinS_HandValues (.values _output) Value))
      (:3
        (Utilities|Struct|SetmembersinS_HandValues (.values _output) Value))
      (:4
        (Utilities|Struct|SetmembersinS_HandValues (.values _output) (* Value -1.0)))
      (:5
        (Utilities|Struct|SetmembersinS_HandValues (.values _output) Value))
      (:6
        (Utilities|Struct|SetmembersinS_HandValues (.values _output) Value)))))

(fn CheckforActiveGesture
  (params (Index :type Integer) (GestureValue :type Float%20%28double-precision%29) (StartingIndex :type Integer) (AmountOfIndexes :type Integer) (HandNR :type Integer))
  (bind _returnvalue (- Index StartingIndex))
  (if (and (>= _returnvalue 0) (< _returnvalue AmountOfIndexes))
    (if (> GestureValue 0.0)
      (Utilities|Struct|SetmembersinS_Hand (Utilities|Array|Get(acopy) (Variables|Default|GetHands) HandNR) (Utilities|Select :Index _returnvalue :Option%200 "NewEnumerator2" :Option%201 "NewEnumerator1" :Option%202 "NewEnumerator0" :Option%203 "NewEnumerator3" :Option%204 "NewEnumerator4" :Option%205 "NewEnumerator5" :Option%206 "NewEnumerator6" :Option%207 "NewEnumerator7")))))

(fn HandleIncomingBundle
  (params (Bundle :type OSC%20Bundle%20Structure%20%28by%20ref%29))
  (bind _returnvalue (Class|OSCManager|GetMessagesfromBundle Bundle))
  (for (_array_element _array_index) _returnvalue
    (bind _values (Class|OSCManager|GetAllFloats _array_element))
    (CallFunction|CheckforActiveGesture _array_index (Utilities|Array|Get(acopy) _values) 1 8)
    (CallFunction|CheckHandParameters _array_index (Utilities|Array|Get(acopy) _values) 9 7)
    (CallFunction|CheckforActiveGesture _array_index (Utilities|Array|Get(acopy) _values) 16 8 1)
    (CallFunction|CheckHandParameters _array_index (Utilities|Array|Get(acopy) _values) 24 7 1)))

(fn Printinfo
  (bind _hands (Variables|Default|GetHands))
  (bind _output (Utilities|Array|Get(acopy) _hands 1))
  (Utilities|FlowControl|Sequence
    (:then_0
      (Development|PrintString (Utilities|String|Append "MESSAGE INDEX: " (Utilities|String|ToString(Integer) (Variables|Default|GetMessageIndex))) true true "(R=1.000000,G=0.863503,B=0.000000,A=1.000000)"))
    (:then_1
      (if (Variables|Default|GetPrint%20Active%20Gesture)
        (Development|PrintString (Utilities|String|Append "ActiveGesture: " (Utilities|String|EnumtoString (.activegesture _output))) true true "(R=0.016571,G=1.000000,B=0.000000,A=1.000000)")))
    (:then_3
      (if (Variables|Default|GetPrint%20Hand%20Values)
        (Development|PrintString (Utilities|String|Append "Hand Active: " (Utilities|String|ToString(Float) (.hand_active (.values _output)))) true true "(R=1.000000,G=0.000000,B=0.982251,A=1.000000)")
        (Development|PrintString (Utilities|String|Append "Velocity: " (Utilities|String|ToString(Float) (.hand_velocity (.values _output)))) true true "(R=1.000000,G=0.000000,B=0.982251,A=1.000000)")
        (Development|PrintString (Utilities|String|Append "X: " (Utilities|String|ToString(Float) (.x (.values _output)))) true true "(R=1.000000,G=0.000000,B=0.982251,A=1.000000)")
        (Development|PrintString (Utilities|String|Append "Y: " (Utilities|String|ToString(Float) (.y (.values _output)))) true true "(R=1.000000,G=0.000000,B=0.982251,A=1.000000)")
        (Development|PrintString (Utilities|String|Append "Z: " (Utilities|String|ToString(Float) (.z (.values _output)))) true true "(R=1.000000,G=0.000000,B=0.982251,A=1.000000)")
        (Development|PrintString (Utilities|String|Append "Rotation: " (Utilities|String|ToString(Float) (.rotation (.values _output)))) true true "(R=1.000000,G=0.000000,B=0.982251,A=1.000000)")
        (Development|PrintString (Utilities|String|Append "Distance: " (Utilities|String|ToString(Float) (.distance (.values _output)))) true true "(R=1.000000,G=0.000000,B=0.982251,A=1.000000)")))))