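; BP_OSC_Receiver turns hand gestures from BP_OSC_Server into telekinesis-like control of a physics-driven object while activated.
; Each tick it copies and rescales hand data, matches each active hand's gesture to levitation, push, pull or gravitation.
; Movement gestures shift an attractor in camera-relative space, and a force proportional to distance pulls the follower after it, with damping lowered when idle.
; Gravitation instead toggles a radial force's strength.
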(event Custom|GravitationStop
  ;[0.6451 0.4224 1 0.5] Effects
  ;;[0.1185 0.4341 0.875 0.5] Gravitation
  (Variables|/Script/Engine.RadialForceComponent|SetForceStrength (Variables|Default|GetRadialForce) 0.0))

(event Custom|Activate
  ;[0.15 0.15 0.15 0.5] BeginPlay, activate, deactivate
  (Variables|InputsGeneral|SetIsActive? true))

(event Custom|Deactivate
  ;[0.15 0.15 0.15 0.5] BeginPlay, activate, deactivate
  (Variables|InputsGeneral|SetIsActive? false))

(event Custom|OnActive
  ;[0.15 0.15 0.15 0.5] OnActive, OnInactive
  (Class|PrimitiveComponent|SetLinearDamping (Variables|Default|GetFollower) 1e+01)
  (if (Variables|Default|GetShouldResetPosition?)
    (CallFunction|SetOverrideVars))
  (Variables|Default|SetShouldResetPosition? false)
  (Timeline|TL_InactiveCooldown PlayFromStart
    (:Finished
      (Variables|Default|SetShouldResetPosition? true))))

(event Custom|OnInactive
  ;[0.15 0.15 0.15 0.5] OnActive, OnInactive
  (CallFunction|StartInactiveCooldown)
  (Class|PrimitiveComponent|SetLinearDamping (Variables|Default|GetFollower) 1.0))

(event Custom|StartInactiveCooldown
  ;[0.15 0.15 0.15 0.5] OnActive, OnInactive
)

(event Custom|StopInactiveCooldown
  ;[0.15 0.15 0.15 0.5] OnActive, OnInactive
)

(event Custom|Levitation
  (params (DeltaSec :type Float%20%28double-precision%29))
  (bind _hands (Variables|ComplexVariables|GetHands))
  (bind _output (Utilities|Array|Get(acopy) _hands))
  ;[0.6451 0.4224 1 0.5] Effects
  ;;[0.1579 0.1578 0.8229 0.5] Levitation
  (Variables|Default|SetCurrentPos (+ (* (Math|Vector|RotateVector (* (Math|Vector|MakeVector (.x (.values _output)) (.y (.values _output)) (.z (.values _output))) (Variables|InputsLevitation|GetLevitationSpeed)) (Variables|Default|GetCamRotation)) DeltaSec) (Variables|Default|GetCurrentPos))))

(event Custom|Push
  (params (DeltaSec :type Float%20%28double-precision%29))
  ;[0.6451 0.4224 1 0.5] Effects
  ;;[0.04924 0.2562 0.8333 0.5] Push and Pull
  (Variables|Default|SetCurrentPos (+ (* (Math|Vector|RotateVector (Math|Vector|MakeVector (Variables|InputsPushing|GetPush%20Speed) 0.0 0.0) (Variables|Default|GetCamRotation)) DeltaSec) (Variables|Default|GetCurrentPos))))

(event Custom|Pull
  (params (DeltaSec :type Float%20%28double-precision%29))
  ;[0.6451 0.4224 1 0.5] Effects
  ;;[0.04924 0.2562 0.8333 0.5] Push and Pull
  (Variables|Default|SetCurrentPos (+ (* (Math|Vector|RotateVector (Math|Vector|MakeVector (* (Variables|InputsPulling|GetPullSpeed) -1.0) 0.0 0.0) (Variables|Default|GetCamRotation)) DeltaSec) (Variables|Default|GetCurrentPos))))

(event Custom|Gravitation
  (params (DeltaSec :type Float%20%28double-precision%29))
  ;[0.6451 0.4224 1 0.5] Effects
  ;;[0.1185 0.4341 0.875 0.5] Gravitation
  (Variables|/Script/Engine.RadialForceComponent|SetForceStrength (Variables|Default|GetRadialForce) (* (Variables|InputsGravitation|GetGravitationForce) 1e+03)))

(event EventBeginPlay
  ;[0.15 0.15 0.15 0.5] BeginPlay, activate, deactivate
  (CallFunction|SetStartVars)
  (bind _returnvalue (Actor|GetActorOfClass "/Game/own/OSC/BP_OSC_Server.BP_OSC_Server_C"))
  (Variables|Default|SetSERVER _returnvalue))

(event EventTick
  (params (DeltaSeconds :type Float%20%28single-precision%29))
  ;[0.15 0.15 0.15 0.5] Event Tick
  (if (Variables|InputsGeneral|GetIsActive?)
    (Variables|Default|SetAnyGestureActive? false)
    (CallFunction|UpdateHandsValues)
    (CallFunction|CreateCameraRotator)
    (for _array_element (Variables|ComplexVariables|GetHands)
      (if (!= (.hand_active (.Values (Utilities|Struct|BreakS_Hand _array_element))) 0.0)
        ;;[0.7268 0.113 0.8646 0.5] Process Effects
        (Utilities|FlowControl|Sequence
          (:then_0
            (if (Utilities|Array|ContainsItem (Variables|InputsLevitation|GetLevitationGestures) (.ActiveGesture (Utilities|Struct|BreakS_Hand _array_element)))
              (Variables|Default|SetAnyGestureActive? true)
              (CallFunction|Levitation DeltaSeconds)))
          (:then_1
            (if (Utilities|Array|ContainsItem (Variables|InputsPushing|GetPushingGestures) (.ActiveGesture (Utilities|Struct|BreakS_Hand _array_element)))
              (Variables|Default|SetAnyGestureActive? true)
              (CallFunction|Push DeltaSeconds)))
          (:then_2
            (if (Utilities|Array|ContainsItem (Variables|InputsPulling|GetPullingGestures) (.ActiveGesture (Utilities|Struct|BreakS_Hand _array_element)))
              (Variables|Default|SetAnyGestureActive? true)
              (CallFunction|Pull DeltaSeconds)))
          (:then_3
            (if (Utilities|Array|ContainsItem (Variables|InputsGravitation|GetGravitationGestures) (.ActiveGesture (Utilities|Struct|BreakS_Hand _array_element)))
              (CallFunction|Gravitation DeltaSeconds)
              (else
                (CallFunction|GravitationStop)))))))
    ;;[0.776 0.002695 0.09426 0.5] Activate Follower
    (if (Variables|Default|GetAnyGestureActive?)
      (CallFunction|OnActive)
      (Transformation|SetWorldLocation (Variables|Default|GetAttractor) (Variables|Default|GetCurrentPos) false false)
      (CallFunction|MoveFollower)
      (else
        (CallFunction|OnInactive)))))

(fn ConstructionScript
  (Components|StaticMesh|SetStaticMesh (Variables|Default|GetAttractor) (Variables|InputsGeneral|GetAttractorMesh))
  (Components|StaticMesh|SetStaticMesh (Variables|Default|GetFollower) (Variables|InputsGeneral|GetFollowerMesh))
  (Rendering|SetVisibility (Variables|Default|GetAttractor) (Variables|InputsGeneral|GetShowAttractor) false)
  (Variables|/Script/Engine.RadialForceComponent|SetRadius (Variables|Default|GetRadialForce) (Variables|InputsGravitation|GetGravitationRange)))

(fn CreateCameraRotator
  (Variables|Default|SetCamRotation (Camera|GetCameraRotation (Variables|Default|GetCAMERA))))

(fn SetStartVars
  (bind _output_get (Variables|Default|SetStartPos (Transformation|GetWorldLocation (Variables|Default|GetAttractor))))
  (Variables|Default|SetCurrentPos _output_get)
  (Variables|Default|SetCAMERA (Game|GetPlayerCameraManager 0)))

(fn SetOverrideVars
  (Variables|Default|SetStartPos (Transformation|GetWorldLocation (Variables|Default|GetFollower))))

(fn UpdateHandsValues
  (bind _locationinputoffset (Variables|InputsLevitation|GetLocationInputOffset))
  (bind _locationinputmultiplier (Variables|InputsLevitation|GetLocationInputMultiplier))
  (bind _output_get (Variables|ComplexVariables|SetHands (Variables|/Game/own/OSC/BP_OSC_Server.BP_OSC_Server_C|GetHands (Variables|Default|GetSERVER))))
  (for (_array_element _array_index) _output_get
    (Utilities|Array|SetArrayElem (Variables|ComplexVariables|GetHands) _array_index (Utilities|Struct|MakeS_Hand (.ActiveGesture (Utilities|Struct|BreakS_Hand _array_element)) (Utilities|Struct|MakeS_HandValues (.hand_active (.Values (Utilities|Struct|BreakS_Hand _array_element))) (.hand_velocity (.Values (Utilities|Struct|BreakS_Hand _array_element))) (* (+ (.x (.Values (Utilities|Struct|BreakS_Hand _array_element))) (.x _locationinputoffset)) (.x _locationinputmultiplier)) (* (+ (.y (.Values (Utilities|Struct|BreakS_Hand _array_element))) (.y _locationinputoffset)) (.y _locationinputmultiplier)) (* (+ (.z (.Values (Utilities|Struct|BreakS_Hand _array_element))) (.z _locationinputoffset)) (.z _locationinputmultiplier)) (.rotation (.Values (Utilities|Struct|BreakS_Hand _array_element))) (.distance (.Values (Utilities|Struct|BreakS_Hand _array_element))))))))

(fn MoveFollower
  (Physics|AddForce (Variables|Default|GetFollower) (* (- (Transformation|GetWorldLocation (Variables|Default|GetAttractor)) (Transformation|GetWorldLocation (Variables|Default|GetFollower))) (Variables|InputsGeneral|GetStrength)) "None" false))